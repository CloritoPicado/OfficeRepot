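; GlobalVariables is a shared Blueprint for the Jousting game that handles pausing and switching player control between the Main pawn and MenuActor.
; Two helper functions possess either pawn.
; FPause opens the Pause widget with cursor and game-and-UI input, hides Main's GUI, pauses its music and the game, resets menu selection state and possesses MenuActor.
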(fn FPossessMain
  (Pawn|Possess (Game|GetPlayerController 0) (Variables|Default|GetMain)))

(fn FPause
  (bind _returnvalue (UserInterface|CreateWidget "/Game/Job_Jousting/Blueprints/Interface/Pause.Pause_C"))
  (UserInterface|Viewport|AddtoViewport _returnvalue 0)
  (Input|SetInputModeGameandUI 0 _returnvalue "DoNotLock" true)
  (Widget|SetVisibility (Variables|/Game/Job_Jousting/Blueprints/Main.Main_C|GetGUI (Variables|Default|GetMain)) "Hidden")
  (Variables|/Script/Engine.PlayerController|SetbShowMouseCursor (Game|GetPlayerController 0) true)
  (Class|AudioComponent|SetPaused (Variables|/Game/Job_Jousting/Blueprints/Main.Main_C|GetBackgroundMusic (Variables|Default|GetMain)) true)
  (Variables|Default|SetMenuID 2)
  (Game|SetGamePaused true)
  (Variables|Default|SetSelection 0)
  (Pawn|Possess (Game|GetPlayerController 0) (Variables|Default|GetMenu_Actor)))

(fn FPossessMenu
  (Pawn|Possess (Game|GetPlayerController 0) (Variables|Default|GetMenu_Actor)))