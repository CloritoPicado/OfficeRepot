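; Input-driven controller actor for the game's main, options and pause menus, creating the MainMenu widget at startup in game mode 0.
; It registers itself in the GlobalVariables game instance, whose MenuID routes navigate, execute and back inputs to MainMenu or PauseUI.
; Up/Down cycle a wrapping shared selection index, while Left/Right step global or music volume in options.
; The Increase flag in FChangeVolume is inverted: true lowers volume.
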(event EventBeginPlay
  (bind _returnvalue (Game|GetPlayerController 0))
  (bind _asglobal_variables (Utilities|Casting|CastToGlobalVariables (Game|GetGameInstance)))
  (bind _output_get (Variables|Default|SetGlobalVariables _asglobal_variables))
  (Variables|/Game/Job_Jousting/Blueprints/GlobalVariables.GlobalVariables_C|SetMenu_Actor _output_get self)
  (if (== 0 (Variables|/Game/Job_Jousting/Blueprints/GlobalVariables.GlobalVariables_C|GetGameMode (Variables|Default|GetGlobalVariables)))
    (bind _returnvalue_2 (UserInterface|CreateWidget "/Game/Job_Jousting/Blueprints/Interface/MainMenu.MainMenu_C"))
    (bind _output_get_2 (Variables|Default|SetMainMenu _returnvalue_2))
    (Variables|/Script/Engine.PlayerController|SetbShowMouseCursor _returnvalue true)
    (Input|SetInputModeGameandUI _returnvalue _output_get_2 "DoNotLock" true)
    (UserInterface|Viewport|AddtoViewport _output_get_2 0)))

(event Collision|EventActorBeginOverlap
  (params (OtherActor :type Actor%20Object%20Reference)))

(event EventTick
  (params (DeltaSeconds :type Float%20%28single-precision%29)))

(event Input|ActionEvents|InputActionB
  (params (Key :type Key%20Structure))
  (:Pressed
    (CallFunction|FEsc "AnyKey")))

(event Input|ActionEvents|InputActionAttack
  (params (Key :type Key%20Structure))
  (:Pressed
    (CallFunction|FExecute)))

(event Input|ActionEvents|InputActionUp
  (params (Key :type Key%20Structure))
  (:Pressed
    (CallFunction|FChangeSelection true)))

(event Input|ActionEvents|InputActionDown
  (params (Key :type Key%20Structure))
  (:Pressed
    (CallFunction|FChangeSelection false)))

(event Input|ActionEvents|InputActionLeft
  (params (Key :type Key%20Structure))
  (:Pressed
    (CallFunction|FChangeVolume true)))

(event Input|ActionEvents|InputActionRight
  (params (Key :type Key%20Structure))
  (:Pressed
    (CallFunction|FChangeVolume false)))

(event Input|KeyboardEvents|Enter
  (params (Key :type Key%20Structure))
  (:Pressed
    (CallFunction|FExecute)))

(event Input|KeyboardEvents|Escape
  (params (Key :type Key%20Structure))
  (:Pressed
    (CallFunction|FEsc "AnyKey")))

(event Input|GamepadEvents|GamepadFaceButtonBottom
  (params (Key :type Key%20Structure))
  (:Pressed
    (CallFunction|FExecute)))

(event Input|GamepadEvents|GamepadSpecialRight
  (params (Key :type Key%20Structure))
  (:Pressed
    (CallFunction|FExecute)))

(fn ConstructionScript)

(fn FChangeSelection
  (params (Positive :type Boolean))
  (bind _globalvariables (Variables|Default|GetGlobalVariables))
  (bind _globalvariables_2 (Variables|Default|GetGlobalVariables))
  (bind _globalvariables_3 (Variables|Default|GetGlobalVariables))
  (switch int (Variables|/Game/Job_Jousting/Blueprints/GlobalVariables.GlobalVariables_C|GetMenuID (Variables|Default|GetGlobalVariables))
    (:0
      (if Positive
        ;[1 1 1] Main Menu
        (if (> (Variables|/Game/Job_Jousting/Blueprints/GlobalVariables.GlobalVariables_C|GetSelection _globalvariables) 0)
          (bind _result (Math|Integer|DecrementInt (Variables|/Game/Job_Jousting/Blueprints/GlobalVariables.GlobalVariables_C|GetSelection _globalvariables))
            (:%20%20
              (Variables|/Game/Job_Jousting/Blueprints/GlobalVariables.GlobalVariables_C|SetSelection _globalvariables _result)))
          (else
            (Variables|/Game/Job_Jousting/Blueprints/GlobalVariables.GlobalVariables_C|SetSelection _globalvariables 5)))
        (elif (< (Variables|/Game/Job_Jousting/Blueprints/GlobalVariables.GlobalVariables_C|GetSelection _globalvariables) 5)
          (bind _result_2 (Math|Integer|IncrementInt (Variables|/Game/Job_Jousting/Blueprints/GlobalVariables.GlobalVariables_C|GetSelection _globalvariables))
            (:%20%20
              (Variables|/Game/Job_Jousting/Blueprints/GlobalVariables.GlobalVariables_C|SetSelection _globalvariables _result_2)))
          (else
            (Variables|/Game/Job_Jousting/Blueprints/GlobalVariables.GlobalVariables_C|SetSelection _globalvariables 0))))
      (Default|FClearAllMain (Variables|Default|GetMainMenu)))
    (:1
      (if Positive
        ;[1 1 1] Options menu
        (if (> (Variables|/Game/Job_Jousting/Blueprints/GlobalVariables.GlobalVariables_C|GetSelection _globalvariables_2) 0)
          (bind _result_3 (Math|Integer|DecrementInt (Variables|/Game/Job_Jousting/Blueprints/GlobalVariables.GlobalVariables_C|GetSelection _globalvariables_2))
            (:%20%20
              (Variables|/Game/Job_Jousting/Blueprints/GlobalVariables.GlobalVariables_C|SetSelection _globalvariables_2 _result_3)))
          (else
            (Variables|/Game/Job_Jousting/Blueprints/GlobalVariables.GlobalVariables_C|SetSelection _globalvariables_2 2)))
        (elif (< (Variables|/Game/Job_Jousting/Blueprints/GlobalVariables.GlobalVariables_C|GetSelection _globalvariables_2) 2)
          (bind _result_4 (Math|Integer|IncrementInt (Variables|/Game/Job_Jousting/Blueprints/GlobalVariables.GlobalVariables_C|GetSelection _globalvariables_2))
            (:%20%20
              (Variables|/Game/Job_Jousting/Blueprints/GlobalVariables.GlobalVariables_C|SetSelection _globalvariables_2 _result_4)))
          (else
            (Variables|/Game/Job_Jousting/Blueprints/GlobalVariables.GlobalVariables_C|SetSelection _globalvariables_2 0))))
      (Default|FClearAllOptions (Variables|Default|GetMainMenu)))
    (:2
      (if Positive
        ;[1 1 1] Pause menu
        (if (> (Variables|/Game/Job_Jousting/Blueprints/GlobalVariables.GlobalVariables_C|GetSelection _globalvariables_3) 0)
          (bind _result_5 (Math|Integer|DecrementInt (Variables|/Game/Job_Jousting/Blueprints/GlobalVariables.GlobalVariables_C|GetSelection _globalvariables_3))
            (:%20%20
              (Variables|/Game/Job_Jousting/Blueprints/GlobalVariables.GlobalVariables_C|SetSelection _globalvariables_3 _result_5)))
          (else
            (Variables|/Game/Job_Jousting/Blueprints/GlobalVariables.GlobalVariables_C|SetSelection _globalvariables_3 3)))
        (elif (< (Variables|/Game/Job_Jousting/Blueprints/GlobalVariables.GlobalVariables_C|GetSelection _globalvariables_3) 3)
          (bind _result_6 (Math|Integer|IncrementInt (Variables|/Game/Job_Jousting/Blueprints/GlobalVariables.GlobalVariables_C|GetSelection _globalvariables_3))
            (:%20%20
              (Variables|/Game/Job_Jousting/Blueprints/GlobalVariables.GlobalVariables_C|SetSelection _globalvariables_3 _result_6)))
          (else
            (Variables|/Game/Job_Jousting/Blueprints/GlobalVariables.GlobalVariables_C|SetSelection _globalvariables_3 0))))
      (Default|FClearPause (Variables|/Game/Job_Jousting/Blueprints/GlobalVariables.GlobalVariables_C|GetPauseUI (Variables|Default|GetGlobalVariables))))))

(fn FChangeVolume
  (params (Increase :type Boolean))
  (bind _globalvariables (Variables|Default|GetGlobalVariables))
  (bind _globalvariables_2 (Variables|Default|GetGlobalVariables))
  (bind _globalvariables_3 (Variables|Default|GetGlobalVariables))
  (bind _mainmenu (Variables|Default|GetMainMenu))
  (bind _mainmenu_2 (Variables|Default|GetMainMenu))
  (bind _selection (Variables|/Game/Job_Jousting/Blueprints/GlobalVariables.GlobalVariables_C|GetSelection _globalvariables))
  (bind _returnvalue (== _selection 1))
  (bind _returnvalue_2 (== _selection 0))
  (if (== (Variables|/Game/Job_Jousting/Blueprints/GlobalVariables.GlobalVariables_C|GetMenuID _globalvariables) 1)
    (if Increase
      ;[1 1 1] Global volume decrease
      (if _returnvalue_2
        (if (> (Variables|/Game/Job_Jousting/Blueprints/GlobalVariables.GlobalVariables_C|GetGlobalVolume _globalvariables_2) 0.2)
          (Variables|/Game/Job_Jousting/Blueprints/GlobalVariables.GlobalVariables_C|SetGlobalVolume _globalvariables_2 (+ (Variables|/Game/Job_Jousting/Blueprints/GlobalVariables.GlobalVariables_C|GetGlobalVolume _globalvariables_2) -0.1))
          (else
            (Variables|/Game/Job_Jousting/Blueprints/GlobalVariables.GlobalVariables_C|SetGlobalVolume _globalvariables_2 0.0)))
        (Default|FRefreshBars _mainmenu)
        (else
          ;[1 1 1] Music volume decrease
          (if _returnvalue
            (if (> (Variables|/Game/Job_Jousting/Blueprints/GlobalVariables.GlobalVariables_C|GetMusicVolume _globalvariables_2) 0.2)
              (Variables|/Game/Job_Jousting/Blueprints/GlobalVariables.GlobalVariables_C|SetMusicVolume _globalvariables_2 (+ (Variables|/Game/Job_Jousting/Blueprints/GlobalVariables.GlobalVariables_C|GetMusicVolume _globalvariables_2) -0.1))
              (else
                (Variables|/Game/Job_Jousting/Blueprints/GlobalVariables.GlobalVariables_C|SetMusicVolume _globalvariables_2 0.0)))
            (Default|FRefreshBars _mainmenu))))
      (else
        ;[1 1 1] Global volume increase
        (if _returnvalue_2
          (if (< (Variables|/Game/Job_Jousting/Blueprints/GlobalVariables.GlobalVariables_C|GetGlobalVolume _globalvariables_3) 1.0)
            (Variables|/Game/Job_Jousting/Blueprints/GlobalVariables.GlobalVariables_C|SetGlobalVolume _globalvariables_3 (+ (Variables|/Game/Job_Jousting/Blueprints/GlobalVariables.GlobalVariables_C|GetGlobalVolume _globalvariables_3) 0.1))
            (else
              (Variables|/Game/Job_Jousting/Blueprints/GlobalVariables.GlobalVariables_C|SetGlobalVolume _globalvariables_3 1.0)))
          (Default|FRefreshBars _mainmenu_2)
          (else
            ;[1 1 1] Music volume increase
            (if _returnvalue
              (if (< (Variables|/Game/Job_Jousting/Blueprints/GlobalVariables.GlobalVariables_C|GetMusicVolume _globalvariables_3) 1.0)
                (Variables|/Game/Job_Jousting/Blueprints/GlobalVariables.GlobalVariables_C|SetMusicVolume _globalvariables_3 (+ (Variables|/Game/Job_Jousting/Blueprints/GlobalVariables.GlobalVariables_C|GetMusicVolume _globalvariables_3) 0.1))
                (else
                  (Variables|/Game/Job_Jousting/Blueprints/GlobalVariables.GlobalVariables_C|SetMusicVolume _globalvariables_3 1.0)))
              (Default|FRefreshBars _mainmenu_2))))))))

(fn FExecute
  (switch int (Variables|/Game/Job_Jousting/Blueprints/GlobalVariables.GlobalVariables_C|GetMenuID (Variables|Default|GetGlobalVariables))
    (:0
      (Default|FExecuteSelection (Variables|Default|GetMainMenu) :!label _label))
    (:1
      (goto _label))
    (:2
      (Default|FExecuteSelection (Variables|/Game/Job_Jousting/Blueprints/GlobalVariables.GlobalVariables_C|GetPauseUI (Variables|Default|GetGlobalVariables)) :!label _label_2))
    (:3
      (goto _label_2))))

(fn FEsc
  (params (Key :type Key%20Structure))
  (bind _globalvariables (Variables|Default|GetGlobalVariables))
  (if (<= (Variables|/Game/Job_Jousting/Blueprints/GlobalVariables.GlobalVariables_C|GetMenuID _globalvariables) 1)
    (if (not (== Key "Gamepad_Special_Right"))
      (Default|FEsc (Variables|Default|GetMainMenu)))
    (else
      (Default|FEsc (Variables|/Game/Job_Jousting/Blueprints/GlobalVariables.GlobalVariables_C|GetPauseUI _globalvariables) Key))))